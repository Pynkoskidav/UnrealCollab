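; Worker_BP is a selectable worker unit that gathers resources and hauls them to storage on right-click orders.
; Clicking a resource starts an AI move-and-gather loop until capacity or depletion, then a trip to NearestStorage; other clicks just move it.
; Drop-off fires CallDropOffResource, with the worker registering itself to the player's resource manager on BeginPlay.
; Carried amounts sit in an array indexed by resource type, shown on camera-facing text.
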(event Custom|CustomEvent_MoveTo
  ;[1 1 1] MoveTo
  (AI|AIMoveTo self "0, 0, 0" (Variables|!Worker|GetcurrentResource) 5.0 false
    (:OnSuccess
      (Development|PrintText "AI move complete" true true "(R=0.000000,G=1.000000,B=0.142064,A=1.000000)")
      (CallFunction|CustomEventGather))
    (:OnFail
      (Development|PrintText "AI Couldn't reach" true true "(R=1.000000,G=0.000000,B=0.028928,A=1.000000)")
      (Variables|!Worker|SetcurrentResource 0))))

(event Custom|CustomEvent_Gather
  (bind _carriedresources (Variables|Default|GetCarriedResources))
  (bind _currentresourcetype (Variables|!Worker|GetcurrentResourceType))
  (bind _returnvalue (Math|Conversions|ToInteger(Byte) _currentresourcetype))
  ;[1 1 1] Gather
  (Utilities|FlowControl|Delay 1.0)
  (Development|PrintText (Utilities|Text|ToText(String) (Utilities|String|Append (Utilities|String|MakeLiteralString "Got") (Utilities|String|EnumtoString (Variables|!Worker|GetcurrentResourceType)))) true true "(R=0.000000,G=1.000000,B=0.000000,A=1.000000)" 0.5)
  (bind _numbergathered (Default|GatherResources (Variables|!Worker|GetcurrentResource)))
  (if (> _numbergathered 0)
    (Utilities|Array|SetArrayElem _carriedresources _returnvalue (+ _numbergathered (Utilities|Array|Get(acopy) _carriedresources _returnvalue)))
    (CallFunction|UpdateUI)
    (Variables|!Worker|SetcurrentCarrying (+ (Variables|!Worker|GetcurrentCarrying) _numbergathered))
    (if (< (Variables|!Worker|GetcurrentCarrying) (Variables|!Worker|GetcarryingCapacity))
      (CallFunction|CustomEventGather)
      (else
        (CallFunction|CustomEventMovefrom)))
    (else
      ;[1 1 1] Stop working, but return held resources
      (Variables|!Worker|SetcurrentResource 0)
      (Variables|!Worker|SetisWorking false)
      (if (> (Variables|!Worker|GetcurrentCarrying) 0)
        (CallFunction|CustomEventMovefrom)))))

(event Custom|CustomEvent_MoveFrom
  (bind _carriedresources (Variables|Default|GetCarriedResources))
  ;[1 1 1] MoveFrom
  (AI|AIMoveTo self "0, 0, 0" (Variables|!Worker|GetnearestStorage) 5.0 false
    (:OnSuccess
      (Development|PrintText "AI move complete" true true "(R=0.000000,G=1.000000,B=0.142064,A=1.000000)")
      (Default|CallDropOffResource _carriedresources)
      (for (_ _array_index) _carriedresources
        (Utilities|Array|SetArrayElem _carriedresources _array_index 0))
      (Variables|!Worker|SetcurrentCarrying 0)
      (CallFunction|UpdateUI)
      (if (Variables|!Worker|GetisWorking)
        (CallFunction|CustomEventMoveto)))
    (:OnFail
      (Development|PrintText "AI Couldn't reach" true true "(R=1.000000,G=0.000000,B=0.028928,A=1.000000)"))))

(event EventBeginPlay
  ;[1 1 1] Begin Play
  ;[1 1 1] Reverse Subscribe Resource Manager
  (bind _asplayer_selectable (Utilities|Casting|CastToPlayer_Selectable (Game|GetPlayerController 0)))
  (Default|CustomEventSubscribe (Variables|/Game/Rob/Selectable/Player/Player_Selectable.Player_Selectable_C|GetManager_Resources _asplayer_selectable) self)
  ;[1 1 1] Resize array match number of resources
  (bind _count (CallFunction|GetResourceTypeCount))
  (Utilities|Array|Resize (Variables|Default|GetCarriedResources) _count))

(event EventTick
  (params (DeltaSeconds :type Float%20%28single-precision%29))
  ;[1 1 1] Tick
  (CallFunction|TextFaceCamera (Variables|Default|GetOxygen))
  (CallFunction|TextFaceCamera (Variables|Default|GetRawMinerals)))

(event EventRightClick
  (params (hit :type Hit%20Result%20Structure))
  (bind (_bblockinghit _binitialoverlap _time _distance _location _impactpoint _normal _impactnormal _physmat _hitactor) (Collision|BreakHitResult hit))
  ;[1 1 1] ISelectable
  (bind _asresource_bp (Utilities|Casting|CastToResource_BP _hitactor)
    (:then
      (Variables|!Worker|SetcurrentResource _asresource_bp)
      (Variables|!Worker|SetcurrentResourceType (Variables|/Game/Rob/Selectable/Classes/NoneSelectable/Resource/Resource_BP.Resource_BP_C|GetresourceType (Variables|!Worker|GetcurrentResource)))
      (Variables|!Worker|SetisWorking true)
      (CallFunction|CustomEventMoveto))
    (:CastFailed
      (Variables|!Worker|SetcurrentResource 0)
      (Variables|!Worker|SetisWorking false)
      (AI|AIMoveTo self _location 0 5.0 false
        (:OnSuccess
          (Development|PrintText "AI move complete" true true "(R=0.000000,G=1.000000,B=0.142064,A=1.000000)"))
        (:OnFail
          (Development|PrintText "AI Couldn't reach" true true "(R=1.000000,G=0.000000,B=0.028928,A=1.000000)"))))))

(fn ConstructionScript
  (|CallParentFunction))

(fn UpdateUI
  (bind _carriedresources (Variables|Default|GetCarriedResources))
  (Rendering|Components|TextRender|SetText (Variables|Default|GetOxygen) (Utilities|Text|ToText(Integer) (Utilities|Array|Get(acopy) _carriedresources)))
  (Rendering|Components|TextRender|SetText (Variables|Default|GetRawMinerals) (Utilities|Text|ToText(Integer) (Utilities|Array|Get(acopy) _carriedresources 1))))