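; Worker_BP is a selectable worker unit that responds to right-click orders by moving or working a resource.
; Right-clicking a Resource_BP stores it and starts a looping AI MoveTo trip between that resource and MainBase, with short pauses at each end.
; Any other click clears the resource and working flag, then moves the worker to the clicked point.
; The loop only handles movement; no resource amounts change here.
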(event Custom|CustomEvent_Working
  (AI|AIMoveTo self "0, 0, 0" (Variables|Default|GetcurrentResource) 5.0 false :!label _label
    (:OnSuccess
      (Utilities|FlowControl|Delay 1.0)
      (AI|AIMoveTo self "0, 0, 0" (Variables|Default|GetmainBase) 5.0 false
        (:OnSuccess
          (Utilities|FlowControl|Delay 0.2)
          (if (Variables|Default|GetisWorking)
            (goto _label)))))))

(event EventRightClick
  (params (hit :type Hit%20Result%20Structure))
  (bind (_bblockinghit _binitialoverlap _time _distance _location _impactpoint _normal _impactnormal _physmat _hitactor) (Collision|BreakHitResult hit))
  (bind _asresource_bp (Utilities|Casting|CastToResource_BP _hitactor)
    (:then
      (Variables|Default|SetcurrentResource _asresource_bp)
      (Variables|Default|SetisWorking true)
      (CallFunction|CustomEventWorking))
    (:CastFailed
      (Variables|Default|SetcurrentResource 0)
      (Variables|Default|SetisWorking false)
      (AI|AIMoveTo self _location 0 5.0 false
        (:OnSuccess
          (Development|PrintText "AI move complete" true true "(R=0.000000,G=1.000000,B=0.142064,A=1.000000)"))
        (:OnFail
          (Development|PrintText "AI Couldn't reach" true true "(R=1.000000,G=0.000000,B=0.028928,A=1.000000)"))))))

(fn ConstructionScript
  (|CallParentFunction))