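; Resource actor that the cursor can hover over and that yields a limited stock of resources when collected.
; Hovering swaps its static mesh between base and highlight materials.
; GetResources subtracts collection ability minus difficulty, clamped between one and the remaining stock, while any remains.
; The returned amount repeats that clamp after the subtraction, so it uses the reduced stock as its maximum.
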(event OnBeginCursorOver(StaticMesh)
  (params (TouchedComponent :type Primitive%20Component%20Object%20Reference))
  (Rendering|Material|SetMaterial (Variables|Default|GetStaticMesh) 0 (Variables|Default|GetmatHighlight)))

(event OnEndCursorOver(StaticMesh)
  (params (TouchedComponent :type Primitive%20Component%20Object%20Reference))
  (Rendering|Material|SetMaterial (Variables|Default|GetStaticMesh) 0 (Variables|Default|GetmatBase)))

(fn ConstructionScript)

(fn GetResources
  (params (CollectionAbility :type Integer))
  (if (> (Variables|Default|GetcurrentResources) 0)
    (Variables|Default|SetcurrentResources (- (Variables|Default|GetcurrentResources) (Math|Integer|Clamp(Integer) (- CollectionAbility (Variables|Default|GetresourceDifficulty)) 1 (Variables|Default|GetcurrentResources))))
    (return (Math|Integer|Clamp(Integer) (- CollectionAbility (Variables|Default|GetresourceDifficulty)) 1 (Variables|Default|GetcurrentResources)))))